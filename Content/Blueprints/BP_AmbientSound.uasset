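; BP_AmbientSound is an actor that plays the level's background music or ambience and lets it be switched by index.
; On BeginPlay it spawns its Sound at the root component's location, keeps the audio component and adjusts it to VolumeLevel.
; The ChangeMusic event maps MusicSelect to one of several hardcoded sound assets, defaulting to the starter cue, and sets it on that same component.
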(event `self.ReceiveBeginPlay`
  (bind _returnvalue (`GameplayStatics.SpawnSoundAtLocation` (`self.Sound`) (`SceneComponent.K2_GetComponentLocation` (`self.DefaultSceneRoot`)) (struct) 1.0 1.0 0.0 null null))
  (bind _output_get (set `self.SoundBeingPlayed` _returnvalue))
  (`AudioComponent.AdjustVolume` _output_get 0.0 (`self.VolumeLevel`) "Linear"))

(event `Change Music`
  (params (MusicSelect :type Integer))
  (switch `int` MusicSelect
    (:`Default`
      (set `self.Sound` "/Game/StarterContent/Audio/Starter_Music_Cue.Starter_Music_Cue" :!label _label))
    (:`0`
      (goto _label))
    (:`1`
      (goto _label))
    (:`2`
      (set `self.Sound` "/Game/Audio/Level2_Cue.Level2_Cue"))
    (:`3`
      (set `self.Sound` "/Game/Audio/CreepSound_Cue.CreepSound_Cue"))
    (:`4`
      (set `self.Sound` "/Game/Cave_Ruins/Audio/SI_Cave_Audio.SI_Cave_Audio"))
    (:`5`
      (set `self.Sound` "/Game/Modular_MedievalTown_WI/Audio/Cue/A_Medieval_Cue.A_Medieval_Cue")))
  (`AudioComponent.SetSound` (`self.SoundBeingPlayed`) (`self.Sound`)))

(fn `UserConstructionScript`)