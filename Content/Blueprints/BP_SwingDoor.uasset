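; BP_SwingDoor is a key-locked door that swings open when the third-person character enters its box trigger and closes when they leave.
; Opening takes one key from the character's KeyCount and plays a Timeline to yaw the mesh up to 90 degrees.
; Exiting an unlocked door returns the key after a short delay, relocks and reverses the Timeline.
; Both moves play offsets of one sound cue; keyless attempts show a locked message with sound.
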(event `self.ReceiveBeginPlay`)

(event `self.Box collision.OnComponentBeginOverlap`
  (params (OverlappedComponent :type "PrimitiveComponent Object Reference") (OtherActor :type "Actor Object Reference") (OtherComp :type "PrimitiveComponent Object Reference") (OtherBodyIndex :type Integer) (bFromSweep :type Boolean) (SweepResult :type "HitResult Structure (by ref)"))
  ;[0 0.1201 1] Open Door
  (bind _asbp_third_person_character_custom (cast `/Game/Blueprints/BP_ThirdPersonCharacterCustom` OtherActor))
  (bind _key_count (`/Game/Blueprints/BP_ThirdPersonCharacterCustom.Key Count` _asbp_third_person_character_custom))
  (if (> _key_count 0)
    (set `/Game/Blueprints/BP_ThirdPersonCharacterCustom.Key Count` (- _key_count 1) _asbp_third_person_character_custom) ; Remove a Key, then open door.
    (bind _returnvalue (`GameplayStatics.SpawnSoundAtLocation` "/Game/Audio/DoorOpenAndClose_Cue.DoorOpenAndClose_Cue" (`SceneComponent.K2_GetComponentLocation` (`self.DefaultSceneRoot`)) (struct) 1.0 1.0 0.0 null null))
    (bind _output_get (set `self.OpenCloseDoor` _returnvalue))
    (`AudioComponent.Play` _output_get 0.3)
    (`AudioComponent.StopDelayed` _output_get 2.0)
    (set `self.DoorUnlocked` true)
    (bind (_direction _newtrack_0) (`Timeline|Timeline` :!via `PlayFromStart` :!label _label)
      (:`Update`
        (`SceneComponent.K2_SetRelativeRotation` (`self.SM_Door`) (`KismetMathLibrary.MakeRotator` 0.0 0.0 (* _newtrack_0 -90.0)) false false)))
    (else
      ;[1 0 0.8008] Door Locked
      (if (not (`self.DoorUnlocked`))
        (`KismetSystemLibrary.PrintString` "Get More Keys! Door is locked" true true (struct :`R` 0.479167 :`G` 0.051103 :`A` 1.0) 5.0)
        (bind _returnvalue_2 (`GameplayStatics.SpawnSoundAtLocation` "/Game/Audio/DoorLockedv2_Cue.DoorLockedv2_Cue" (`SceneComponent.K2_GetComponentLocation` (`self.DefaultSceneRoot`)) (struct) 1.0 1.0 0.0 null null))
        (bind _output_get_2 (set `self.OpenCloseDoor` _returnvalue_2))
        (`AudioComponent.Play` _output_get_2 0.0)
        (`AudioComponent.StopDelayed` _output_get_2 2.0)))))

(event `self.Box collision.OnComponentEndOverlap`
  (params (OverlappedComponent :type "PrimitiveComponent Object Reference") (OtherActor :type "Actor Object Reference") (OtherComp :type "PrimitiveComponent Object Reference") (OtherBodyIndex :type Integer))
  ;[1 0 0.003775] Close Door
  (bind _asbp_third_person_character_custom (cast `/Game/Blueprints/BP_ThirdPersonCharacterCustom` OtherActor))
  (if (`self.DoorUnlocked`)
    (`KismetSystemLibrary.Delay` 0.2)
    (set `/Game/Blueprints/BP_ThirdPersonCharacterCustom.Key Count` (+ (`/Game/Blueprints/BP_ThirdPersonCharacterCustom.Key Count` _asbp_third_person_character_custom) 1) _asbp_third_person_character_custom) ; Remove a Key, then open door.
    (bind _returnvalue (`GameplayStatics.SpawnSoundAtLocation` "/Game/Audio/DoorOpenAndClose_Cue.DoorOpenAndClose_Cue" (`SceneComponent.K2_GetComponentLocation` (`self.DefaultSceneRoot`)) (struct) 1.0 1.0 0.0 null null))
    (bind _output_get (set `self.OpenCloseDoor` _returnvalue))
    (`AudioComponent.Play` _output_get 3.2)
    (`AudioComponent.StopDelayed` _output_get 2.0)
    (set `self.DoorUnlocked` false)
    (goto _label :!via `ReverseFromEnd`)))

(fn `UserConstructionScript`)