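; Checkpoint zone actor that saves the player's progress when the custom third-person character overlaps its cylinder.
; Each such overlap calls SaveCheckpoint on the character and plays a checkpoint sound at the actor, with a delayed stop.
; The glow ring starts at zero scale; on first activation a timeline grows it vertically to full size, and a GlowVis flag prevents the animation from replaying.
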(event `self.ReceiveBeginPlay`
  (`SceneComponent.SetWorldScale3D` (`self.SM_FX_Glow_Ring_01`) (0.0 0.0 0.0)))

(event `self.ReceiveTick`
  (params (DeltaSeconds :type "Float (single-precision)")))

(event `self.Cylinder.OnComponentBeginOverlap`
  (params (OverlappedComponent :type "PrimitiveComponent Object Reference") (OtherActor :type "Actor Object Reference") (OtherComp :type "PrimitiveComponent Object Reference") (OtherBodyIndex :type Integer) (bFromSweep :type Boolean) (SweepResult :type "HitResult Structure (by ref)"))
  (bind _asbp_third_person_character_custom (cast `/Game/Blueprints/BP_ThirdPersonCharacterCustom` OtherActor))
  (`/Game/Blueprints/BP_ThirdPersonCharacterCustom.Save Checkpoint` _asbp_third_person_character_custom)
  (bind _returnvalue (`GameplayStatics.SpawnSoundAtLocation` "/Game/Audio/CheckPoint_Cue.CheckPoint_Cue" (`SceneComponent.K2_GetComponentLocation` (`self.DefaultSceneRoot`)) (struct) 1.0 1.0 0.0 null null))
  (`AudioComponent.Play` _returnvalue 0.0)
  (`AudioComponent.StopDelayed` _returnvalue 5.0)
  (if (not (`self.glowVis`))
    (bind (_direction _newtrack_0) (`Timeline|Timeline_0` :!via `PlayFromStart`)
      (:`Update`
        (`SceneComponent.SetWorldScale3D` (`self.SM_FX_Glow_Ring_01`) (`KismetMathLibrary.MakeVector` 0.45 0.45 (`KismetMathLibrary.Lerp` 0.0 0.45 _newtrack_0)))
        (set `self.glowVis` true)))))

(fn `UserConstructionScript`)