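; Key-locked stone door that rolls open when the player character enters its collision box.
; DoorCode indexes the character's key-count array; a positive count consumes a key, plays stone audio and runs a timeline that rotates and shifts the door mesh.
; Without a key, a still-locked door prints a warning and plays a locked sound.
; The closing and key-refund logic is disconnected, so the door never closes.
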(event `self.ReceiveBeginPlay`)

(event `self.Box collision.OnComponentBeginOverlap`
  (params (OverlappedComponent :type "PrimitiveComponent Object Reference") (OtherActor :type "Actor Object Reference") (OtherComp :type "PrimitiveComponent Object Reference") (OtherBodyIndex :type Integer) (bFromSweep :type Boolean) (SweepResult :type "HitResult Structure (by ref)"))
  (bind _sm_door (`self.SM_Door`))
  ;[0 0.1201 1] Open Door
  (bind _asbp_third_person_character_custom (cast `/Game/Blueprints/BP_ThirdPersonCharacterCustom` OtherActor))
  (bind _canopen (`self.doorCoded` _asbp_third_person_character_custom))
  (if _canopen
    (`self.removeKey` _asbp_third_person_character_custom)
    (bind _returnvalue (`GameplayStatics.SpawnSoundAtLocation` "/Game/Audio/Stones_Cue.Stones_Cue" (`SceneComponent.K2_GetComponentLocation` (`self.DefaultSceneRoot`)) (struct) 1.0 1.0 0.0 null null))
    (bind _output_get (set `self.OpenCloseDoor` _returnvalue))
    (`AudioComponent.Play` _output_get 22.0)
    (`AudioComponent.StopDelayed` _output_get 3.0)
    (set `self.DoorUnlocked` true)
    (bind (_direction _newtrack_0) (`Timeline|Timeline` :!via `PlayFromStart`)
      (:`Update`
        (`SceneComponent.K2_SetRelativeRotation` _sm_door (`KismetMathLibrary.MakeRotator` 90.0 (* _newtrack_0 -90.0) 90.0) false false)
        (`SceneComponent.K2_AddRelativeLocation` _sm_door (`KismetMathLibrary.MakeVector` 0.0 (* _newtrack_0 10.0)) false false)))
    (else
      ;[1 0 0.8008] Door Locked
      (if (not (`self.DoorUnlocked`))
        (`KismetSystemLibrary.PrintString` "Get More Keys! Door is locked" true true (struct :`R` 0.479167 :`G` 0.051103 :`A` 1.0) 5.0)
        (bind _returnvalue_2 (`GameplayStatics.SpawnSoundAtLocation` "/Game/Audio/DoorLockedv2_Cue.DoorLockedv2_Cue" (`SceneComponent.K2_GetComponentLocation` (`self.DefaultSceneRoot`)) (struct) 1.0 1.0 0.0 null null))
        (bind _output_get_2 (set `self.OpenCloseDoor` _returnvalue_2))
        (`AudioComponent.Play` _output_get_2 0.0)
        (`AudioComponent.StopDelayed` _output_get_2 2.0)))))

(event `self.Box collision.OnComponentEndOverlap`
  (params (OverlappedComponent :type "PrimitiveComponent Object Reference") (OtherActor :type "Actor Object Reference") (OtherComp :type "PrimitiveComponent Object Reference") (OtherBodyIndex :type Integer))
  ;[1 0 0.003775] Close Door
)

(fn `addKey`
  (params (char :type "/Game/Blueprints/BP_ThirdPersonCharacterCustom Object Reference"))
  (bind _doorcode (`self.doorCode`))
  (bind _key (break `/Game/Blueprints/structs/keys` (`/Game/Blueprints/BP_ThirdPersonCharacterCustom.keys` char)))
  (for (_array_element _array_index) _key
    (if (== _array_index _doorcode)
      (`KismetArrayLibrary.Array_Set` _key _doorcode (+ _array_element 1)))))

(fn `doorCoded`
  (params (Char :type "/Game/Blueprints/BP_ThirdPersonCharacterCustom Object Reference"))
  (returns (canOpen :type Boolean))
  (for (_array_element _array_index) (`.key_14_78B33AFB4BA0F36918BA8A8CBAF46170` (break `/Game/Blueprints/structs/keys` (`/Game/Blueprints/BP_ThirdPersonCharacterCustom.keys` Char)))
    (if (== _array_index (`self.doorCode`))
      (return (> _array_element 0)))))

(fn `removeKey`
  (params (char :type "/Game/Blueprints/BP_ThirdPersonCharacterCustom Object Reference"))
  (bind _doorcode (`self.doorCode`))
  (bind _key (break `/Game/Blueprints/structs/keys` (`/Game/Blueprints/BP_ThirdPersonCharacterCustom.keys` char)))
  (for (_array_element _array_index) _key
    (if (== _array_index _doorcode)
      (`KismetArrayLibrary.Array_Set` _key _doorcode (- _array_element 1))))
  (`KismetSystemLibrary.PrintString` (`KismetStringLibrary.Concat_StrStr` "The Player has " (`KismetStringLibrary.Conv_IntToString` 0) " key(s) of type: " (`KismetStringLibrary.Conv_IntToString` 0)) true true (struct :`G` 0.66 :`B` 1.0 :`A` 1.0) 5.0))

(fn `UserConstructionScript`)