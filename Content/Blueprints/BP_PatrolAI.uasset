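; BP_PatrolAI is a patrolling AI character that varies its mesh and walk speed randomly at spawn.
; BeginPlay gathers actors tagged PatrolPoint_TestMap and shuffles them into its own route.
; GoToPatrolPoint loops through that route with AIMoveTo, advancing after a short delay on success or failure and wrapping at the end.
; A separate GoToPlayer event chases player 0, repeating only on success, but nothing in this graph calls it.
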(event `self.ReceiveBeginPlay`
  (`SkeletalMeshComponent.SetSkeletalMeshAsset` (`self.Mesh`) (`|GetArrayItem` (`self.New Mesh`) (`KismetMathLibrary.RandomInteger` 4)))
  (bind _outactors (`GameplayStatics.GetAllActorsOfClassWithTag` "/Script/Engine.Actor" "PatrolPoint_TestMap"))
  (bind _output_get (set `self.PatrolPoints` _outactors))
  (`KismetArrayLibrary.Array_Shuffle` _output_get)
  (`KismetSystemLibrary.PrintString` (`KismetStringLibrary.Concat_StrStr` "There are " (`KismetStringLibrary.Conv_IntToString` (`KismetArrayLibrary.Array_Length` _output_get)) " many patrol points"))
  (set `CharacterMovementComponent.MaxWalkSpeed` (`KismetMathLibrary.Conv_IntToDouble` (* (`KismetMathLibrary.RandomIntegerInRange` 8 12) 25)) (`self.CharacterMovement`))
  (`self.GoToPatrolPoint`))

(event `GoToPatrolPoint`
  (bind _output (`|GetArrayItem` (`self.PatrolPoints`) (`self.PPIndex`)))
  (`|AIMoveTo` self (`self.K2_GetActorLocation` _output) null 100.0
    (:`OnSuccess`
      (`KismetSystemLibrary.PrintString` "Arivived at destination" true true (struct :`G` 0.66 :`B` 1.0 :`A` 1.0) 5.0))
    (:`OnFail`
      (`KismetSystemLibrary.PrintString` (`KismetStringLibrary.Concat_StrStr` "Failed to arrive at: " (`KismetSystemLibrary.GetDisplayName` _output)) true true (struct :`G` 0.66 :`B` 1.0 :`A` 1.0) 5.0)))
  (bind _result (`/Engine/EditorBlueprintResources/StandardMacros.IncrementInt` (`self.PPIndex`))
    (:`  `
      (if (>= _result (`KismetArrayLibrary.Array_Length` (stale `self.ReceiveBeginPlay` _output_get)))
        (set `self.PPIndex` 0))
      (`KismetSystemLibrary.Delay` 0.2)
      (`self.GoToPatrolPoint`))))

(event `GoToPlayer`
  (`|AIMoveTo` self (0.0 0.0 0.0) (`GameplayStatics.GetPlayerCharacter` 0) 0.0
    (:`OnSuccess`
      (`KismetSystemLibrary.PrintString` "Arivived at destination" true true (struct :`G` 0.66 :`B` 1.0 :`A` 1.0) 5.0)
      (`KismetSystemLibrary.Delay` 1.0)
      (`self.GoToPlayer`))
    (:`OnFail`
      (`KismetSystemLibrary.PrintString` "Failed to arrive" true true (struct :`G` 0.66 :`B` 1.0 :`A` 1.0) 5.0))))

(fn `UserConstructionScript`)